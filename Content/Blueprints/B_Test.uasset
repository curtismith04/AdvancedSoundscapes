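; Test actor that builds a grid of instanced cubes and applies a three-band, distance-based LOD effect relative to the player.
; The construction script spaces instances by mesh bounds plus offsets, and BeginPlay creates a dynamic material and binds to the character's K-press event.
; UpdateCubes sets each instance's height by distance band, dirtying render state only on the last.
; Emissive color is written to one shared material, so it is not per-instance.
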(event `self.ReceiveBeginPlay`
  (bind _returnvalue (`PrimitiveComponent.CreateDynamicMaterialInstance` (`self.InstancedStaticMesh`) 0 "/Game/Materials/M_CubeBase_LOD.M_CubeBase_LOD" "CubeMaterial"))
  (set `self.DynamicMaterial` _returnvalue)
  (bind _asbp_third_person_character (cast `/Game/ThirdPersonTemplate/ThirdPerson/Blueprints/BP_ThirdPersonCharacter` (`GameplayStatics.GetPlayerCharacter` 0)))
  (set `self.As BP Third Person Character` _asbp_third_person_character)
  (add `/Game/ThirdPersonTemplate/ThirdPerson/Blueprints/BP_ThirdPersonCharacter.OnKPressed` _asbp_third_person_character (`|CreateDelegate` :!event `Update Cubes`)))

(event `self.ReceiveTick`
  (params (DeltaSeconds :type "Float (single-precision)")))

(event `Update Cubes`
  (bind _instancedstaticmesh (`self.InstancedStaticMesh`))
  (bind _instancedstaticmesh_2 (`self.InstancedStaticMesh`))
  (bind _returnvalue (- (`InstancedStaticMeshComponent.GetInstanceCount` _instancedstaticmesh) 1))
  (for _index (range (+ _returnvalue 1))
    (set `self.Mark Render State Dirty` (== _index _returnvalue))
    (set `self.DistanceToPlayer` (`KismetMathLibrary.Vector_Distance` (.location (`InstancedStaticMeshComponent.GetInstanceTransform` _instancedstaticmesh _index true)) (`self.K2_GetActorLocation` (`self.As BP Third Person Character`))))
    (if (`KismetMathLibrary.InRange_FloatFloat` (`self.DistanceToPlayer`) 0.0 (`self.LOD1_Range`))
      (`MaterialInstanceDynamic.SetVectorParameterValue` (`self.DynamicMaterial`) "Emissive" (struct :`R` 0.771409 :`G` 10.0 :`A` 1.0))
      (set `self.Delta Location Z` 0.0)
      (bind _outinstancetransform (`InstancedStaticMeshComponent.GetInstanceTransform` _instancedstaticmesh_2 _index false))
      (`InstancedStaticMeshComponent.UpdateInstanceTransform` _instancedstaticmesh_2 _index (`KismetMathLibrary.MakeTransform` (`KismetMathLibrary.MakeVector` (.x (.location _outinstancetransform)) (.y (.location _outinstancetransform)) (`self.Delta Location Z`)) (.rotation _outinstancetransform) (.scale _outinstancetransform)) false (`self.Mark Render State Dirty`) false :!label _label)
      (else
        (`|ExecutionSequence`
          (:`then_0`
            (if (`KismetMathLibrary.InRange_FloatFloat` (`self.DistanceToPlayer`) (`self.LOD1_Range`) (`self.LOD2_Range`))
              (`MaterialInstanceDynamic.SetVectorParameterValue` (`self.DynamicMaterial`) "Emissive" (struct :`R` 8.299813 :`B` 10.0 :`A` 1.0))
              (set `self.Delta Location Z` 50.0)
              (goto _label)
              (else
                (`|ExecutionSequence`
                  (:`then_0`
                    (if (> (`self.DistanceToPlayer`) (`self.LOD2_Range`))
                      (`MaterialInstanceDynamic.SetVectorParameterValue` (`self.DynamicMaterial`) "Emissive" (struct :`R` 50.0 :`G` 22.86644 :`A` 1.0))
                      (set `self.Delta Location Z` 100.0)
                      (goto _label)))
                  (:`then_1`)))))
          (:`then_1`))))))

(fn `UserConstructionScript`
  (bind (_min _max) (`StaticMeshComponent.GetLocalBounds` (`self.InstancedStaticMesh`)))
  (bind (_returnvalue_x _returnvalue_y) (`KismetMathLibrary.BreakVector` (- _max _min)))
  (for _index (range (`self.Rows`))
    (for _index_2 (range (`self.Columns`))
      (`InstancedStaticMeshComponent.AddInstance` (`self.InstancedStaticMesh`) (`KismetMathLibrary.Conv_VectorToTransform` (`KismetMathLibrary.MakeVector` (* _index (+ (`self.XOffset`) _returnvalue_x)) (* _index_2 (+ (`self.YOffset`) _returnvalue_y)))) false))))