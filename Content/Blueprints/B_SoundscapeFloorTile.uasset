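; Floor tile actor that changes emissive colour and height according to its distance from the player character, in three LOD bands.
; Tick compares the distance with two LOD ranges, setting a dynamic material's colour and the cube's absolute world Z, higher when farther.
; DoOnce gates limit repeat updates, but their nested resets leave the far band firing only once and the middle re-arming only from the far band.
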(event `self.ReceiveBeginPlay`
  (bind _returnvalue (`PrimitiveComponent.CreateDynamicMaterialInstance` (`self.Cube`) 0 "/Game/Materials/M_CubeBase_LOD.M_CubeBase_LOD" "CubeMaterial"))
  (set `self.DynamicMaterial` _returnvalue)
  (bind _asbp_third_person_character (cast `/Game/ThirdPersonTemplate/ThirdPerson/Blueprints/BP_ThirdPersonCharacter` (`GameplayStatics.GetPlayerCharacter` 0)))
  (set `self.As BP Third Person Character` _asbp_third_person_character))

(event `self.ReceiveTick`
  (params (DeltaSeconds :type "Float (single-precision)"))
  (bind _cube (`self.Cube`))
  (bind (_returnvalue_x _returnvalue_y) (`KismetMathLibrary.BreakVector` (`SceneComponent.K2_GetComponentLocation` _cube)))
  (set `self.DistanceToPlayer` (`self.GetDistanceTo` self (`self.As BP Third Person Character`)))
  (if (`KismetMathLibrary.InRange_FloatFloat` (`self.DistanceToPlayer`) 0.0 (`self.LOD1_Range`))
    (`/Engine/EditorBlueprintResources/StandardMacros.DoOnce` false :!label _label
      (:`Completed`
        (`MaterialInstanceDynamic.SetVectorParameterValue` (`self.DynamicMaterial`) "Emissive" (struct :`R` 0.771409 :`G` 10.0 :`A` 1.0))
        (set `self.Delta Location Z` 0.0)))
    (else
      (`|ExecutionSequence`
        (:`then_0`
          (if (`KismetMathLibrary.InRange_FloatFloat` (`self.DistanceToPlayer`) (`self.LOD1_Range`) (`self.LOD2_Range`))
            (`/Engine/EditorBlueprintResources/StandardMacros.DoOnce` false :!label _label_2
              (:`Completed`
                (`MaterialInstanceDynamic.SetVectorParameterValue` (`self.DynamicMaterial`) "Emissive" (struct :`R` 8.299813 :`B` 10.0 :`A` 1.0))
                (set `self.Delta Location Z` 50.0)))
            (else
              (`|ExecutionSequence`
                (:`then_0`
                  (if (> (`self.DistanceToPlayer`) (`self.LOD2_Range`))
                    (`/Engine/EditorBlueprintResources/StandardMacros.DoOnce` false :!label _label_3
                      (:`Completed`
                        (`MaterialInstanceDynamic.SetVectorParameterValue` (`self.DynamicMaterial`) "Emissive" (struct :`R` 50.0 :`G` 22.86644 :`A` 1.0))
                        (set `self.Delta Location Z` 100.0)))
                    (else
                      (goto _label_3 :!via `Reset`))))
                (:`then_1`
                  (goto _label_2 :!via `Reset`))))))
        (:`then_1`
          (goto _label :!via `Reset`)))))
  (`SceneComponent.K2_SetWorldTransform` _cube (`KismetMathLibrary.MakeTransform` (`KismetMathLibrary.MakeVector` _returnvalue_x _returnvalue_y (`self.Delta Location Z`))) false false))

(fn `UserConstructionScript`)